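; GM_Main is the game manager for CrossingPoint, handling startup UI and the link to the player's chicken.
; On BeginPlay it shows a splash screen for a few seconds, then swaps in the HUD and passes itself to it.
; It then casts the player character to BP_Chicken, stores it and registers itself on it.
; Every Tick it has the HUD refresh its counter text.
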(event EventBeginPlay
  (bind _returnvalue (UserInterface|CreateWidget "/Game/CrossingPoint/Blueprints/BP_SplashScreen.BP_SplashScreen_C"))
  (UserInterface|Viewport|AddtoViewport _returnvalue 0)
  (Utilities|FlowControl|Delay 3.5)
  (Widget|RemovefromParent _returnvalue)
  (bind _returnvalue_2 (UserInterface|CreateWidget "/Game/CrossingPoint/Blueprints/BP_Hud.BP_Hud_C"))
  (UserInterface|Viewport|AddtoViewport _returnvalue_2 0)
  (Variables|/Game/CrossingPoint/Blueprints/BP_Hud.BP_Hud_C|SetGame%20Manager _returnvalue_2 self)
  (bind _output_get (Variables|Default|SetHUD%20Widget _returnvalue_2))
  (Default|UpdateCounterText _output_get)
  (bind _asbp_chicken (Utilities|Casting|CastToBP_Chicken (Game|GetPlayerCharacter 0)))
  (bind _output_get_2 (Variables|Default|SetPlayer _asbp_chicken))
  (Variables|/Game/CrossingPoint/Blueprints/BP_Chicken.BP_Chicken_C|SetGame%20Manager%20Connector _output_get_2 self))

(event EventTick
  (params (DeltaSeconds :type Float%20%28single-precision%29))
  (Default|UpdateCounterText (Variables|Default|GetHUD%20Widget)))

(fn ConstructionScript)