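; Spawner actor that builds a chain of BP_MapSegment actors starting at the player pawn's location.
; On BeginPlay it spawns an initial batch, placing each new segment at the SpawnPoint of the previous one, tracked as NewestSegment.
; Each segment receives a SegmentSpawner reference back to this actor, and SpawnSegmentAtSpawnPoint extends the chain by one segment.
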(event EventBeginPlay
  (CallFunction|SpawnInitialSegments))

(event Collision|EventActorBeginOverlap
  (params (OtherActor :type Actor%20Object%20Reference)))

(event EventTick
  (params (DeltaSeconds :type Float%20%28single-precision%29)))

(fn ConstructionScript)

(fn SpawnMapSegment
  (params (SpawnLocation :type Vector))
  (bind _returnvalue (Game|SpawnActorfromClass "/Game/CrossingPoint/Blueprints/BP_MapSegment.BP_MapSegment_C" (Math|Conversions|ToTransform(Vector) SpawnLocation) "Undefined" 0 0))
  (bind _output_get (Variables|Default|SetNewestSegment _returnvalue))
  (Variables|/Game/CrossingPoint/Blueprints/BP_MapSegment.BP_MapSegment_C|SetSegmentSpawner _output_get self))

(fn SpawnSegmentatSpawnPoint
  (CallFunction|SpawnMapSegment (Transformation|GetWorldLocation (Variables|/Game/CrossingPoint/Blueprints/BP_MapSegment.BP_MapSegment_C|GetSpawnPoint (Variables|Default|GetNewestSegment)))))

(fn SpawnInitialSegments
  (for _index (range 0 6)
    (Utilities|IsValid (Variables|Default|GetNewestSegment)
      (:Is%20Valid
        (CallFunction|SpawnSegmentatSpawnPoint))
      (:Is%20Not%20Valid
        (CallFunction|SpawnMapSegment (Transformation|GetActorLocation (Game|Player|GetPlayerPawn 0)))))))