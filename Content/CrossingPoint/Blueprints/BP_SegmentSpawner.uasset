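; Spawner actor that lays out terrain segments of a crossing level in a line along the world Y axis.
; SpawnSegment randomly spawns a water, grass, road or rail segment, offset by a fixed stride times SegmentCount, then increments that count.
; Each segment receives a reference back to the spawner; BeginPlay spawns only one, and no other call to SpawnSegment is made here.
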(event EventBeginPlay
  (CallFunction|SpawnSegment))

(event Collision|EventActorBeginOverlap
  (params (OtherActor :type Actor%20Object%20Reference)))

(event EventTick
  (params (DeltaSeconds :type Float%20%28single-precision%29)))

(fn ConstructionScript)

(fn SpawnSegment
  (bind _segment_count (Variables|Default|Getsegment_count))
  (bind _returnvalue (* "0,3200.000000, 0" _segment_count))
  (bind _returnvalue_2 (Math|Transform|MakeTransform _returnvalue))
  (switch int (Math|Random|RandomIntegerinRange 0 3)
    (:0
      (bind _returnvalue_3 (Game|SpawnActorfromClass "/Game/CrossingPoint/Blueprints/BP_Water.BP_Water_C" _returnvalue_2 "Undefined" 0 0))
      (Math|Integer|IncrementInt (Variables|Default|Getsegment_count)
        (:%20%20
          (bind _output_get (Variables|Default|SetNewWater _returnvalue_3))
          (Variables|/Game/CrossingPoint/Blueprints/BP_Water.BP_Water_C|SetSegmentSpawner _output_get self))))
    (:1
      (bind _returnvalue_4 (Game|SpawnActorfromClass "/Game/CrossingPoint/Blueprints/BP_Grass.BP_Grass_C" _returnvalue_2 "Undefined" 0 0))
      (Math|Integer|IncrementInt (Variables|Default|Getsegment_count)
        (:%20%20
          (bind _output_get_2 (Variables|Default|SetNewGrass _returnvalue_4))
          (Variables|/Game/CrossingPoint/Blueprints/BP_Grass.BP_Grass_C|SetSegmentSpawner _output_get_2 self))))
    (:2
      (bind _returnvalue_5 (Game|SpawnActorfromClass "/Game/CrossingPoint/Blueprints/BP_Road.BP_Road_C" _returnvalue_2 "Undefined" 0 0))
      (Math|Integer|IncrementInt (Variables|Default|Getsegment_count)
        (:%20%20
          (bind _output_get_3 (Variables|Default|SetNewRoad _returnvalue_5))
          (Variables|/Game/CrossingPoint/Blueprints/BP_Road.BP_Road_C|SetSegmentSpawner _output_get_3 self))))
    (:3
      (bind _returnvalue_6 (Game|SpawnActorfromClass "/Game/CrossingPoint/Blueprints/BP_Rail.BP_Rail_C" _returnvalue_2 "Undefined" 0 0))
      (Math|Integer|IncrementInt (Variables|Default|Getsegment_count)
        (:%20%20
          (bind _output_get_4 (Variables|Default|SetNewRail _returnvalue_6))
          (Variables|/Game/CrossingPoint/Blueprints/BP_Rail.BP_Rail_C|SetSegmentSpawner _output_get_4 self))))))